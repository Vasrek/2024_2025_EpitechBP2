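; Falling platform that drops shortly after the player steps on it, then resets for reuse.
; Player overlap with the box collider, after a delay, turns the cube red, plays a warning sound, then enables physics simulation so it falls.
; After a few seconds it disables physics, teleports back to the transform saved at BeginPlay and restores its material.
; HasBeenUsed blocks retriggering but is set only after the first delay.
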(event OnComponentBeginOverlap(BoxCollider)
  (params (OverlappedComponent :type Primitive%20Component%20Object%20Reference) (OtherActor :type Actor%20Object%20Reference) (OtherComp :type Primitive%20Component%20Object%20Reference) (OtherBodyIndex :type Integer) (bFromSweep :type Boolean) (SweepResult :type Hit%20Result%20Structure%20%28by%20ref%29))
  ;[1 1 1] Check if the player entered in the box collision
  (if (and (== OtherActor (Game|GetPlayerCharacter 0)) (not (Variables|Default|GetHasBeenUsed?)))
    (Utilities|FlowControl|Delay 1.0)
    (CallFunction|BeforeFallingPlatform)))

(event Custom|RespawnPlatform
  (bind _cubemesh (Variables|Default|GetCubeMesh))
  ;[1 1 1] Disable physics / teleport platform back to default / switch material to default
  (Physics|SetSimulatePhysics _cubemesh false)
  (Transformation|SetWorldTransform _cubemesh (Variables|Default|GetDefaultLocation) false true)
  (Rendering|Material|SetMaterial (Variables|Default|GetCubeMesh) 0 "/Engine/BasicShapes/BasicShapeMaterial.BasicShapeMaterial")
  (Variables|Default|SetHasBeenUsed? false))

(event Custom|BeforeFallingPlatform
  ;[1 1 1] Change material / Play sound
  (Variables|Default|SetHasBeenUsed? true)
  (Rendering|Material|SetMaterial (Variables|Default|GetCubeMesh) 0 "/AnimationSharing/AnimSharingRed.AnimSharingRed")
  (Audio|PlaySound2D "/Engine/VREditor/Sounds/UI/Camera_Shutter.Camera_Shutter" 1.0 1.0 0.0 0 0)
  (Utilities|FlowControl|Delay 0.5)
  (CallFunction|MakethePlatformFalls))

(event Custom|MakeThePlatformFalls
  ;[1 1 1] Simulate physics / After 5 second call respawn
  (Physics|SetSimulatePhysics (Variables|Default|GetCubeMesh) true)
  (Utilities|FlowControl|Delay 5.0)
  (CallFunction|RespawnPlatform))

(event EventBeginPlay
  ;[1 0 0.03196] Save platform tranasform
  (Variables|Default|SetDefaultLocation (Transformation|GetWorldTransform (Variables|Default|GetCubeMesh))))

(fn ConstructionScript)